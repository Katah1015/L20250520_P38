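; BP_P38 is a player-controlled P-38 aircraft with simple arcade flight driven by input axes.
; Pitch and Roll apply frame-time-scaled local rotations, while Engine acts as a throttle that accumulates a clamped, non-negative speed for forward local movement.
; BeginPlay registers both propeller meshes with BPSceneRotator, and Move feeds the current speed to it as MotorSpeed, printing that value for debugging.
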(event `self.ReceiveBeginPlay`
  (bind _scenecomponents (`/Game/Blueprints/BP_SceneRotator.SceneComponents` (`self.BP_SceneRotator`)))
  (`KismetArrayLibrary.Array_Add` _scenecomponents (`self.SM_P38_Propeller_Left`))
  (`KismetArrayLibrary.Array_Add` _scenecomponents (`self.SM_P38_Propeller_Right`)))

(event `InputAxis|Engine`
  (params (AxisValue :type "Float (single-precision)"))
  (`self.Move` (`KismetMathLibrary.FClamp` AxisValue -1.0)))

(event `InputAxis|Pitch`
  (params (AxisValue :type "Float (single-precision)"))
  (`self.K2_AddActorLocalRotation` (`KismetMathLibrary.MakeRotator` 0.0 (* (`KismetMathLibrary.FClamp` AxisValue -1.0) (`GameplayStatics.GetWorldDeltaSeconds`) 60.0))))

(event `InputAxis|Roll`
  (params (AxisValue :type "Float (single-precision)"))
  (`self.K2_AddActorLocalRotation` (`KismetMathLibrary.MakeRotator` (* (`KismetMathLibrary.FClamp` AxisValue -1.0) (`GameplayStatics.GetWorldDeltaSeconds`) 60.0))))

(fn `Move`
  (params (Speed :type "Float (double-precision)"))
  (`self.K2_AddActorLocalOffset` (`KismetMathLibrary.MakeVector` (* (`GameplayStatics.GetWorldDeltaSeconds`) (`self.MoveSpeed`))))
  (bind _output_get (set `self.MoveSpeed` (`KismetMathLibrary.FClamp` (+ (`self.MoveSpeed`) (* Speed 10.0)) 0.0 1000.0)))
  (bind _output_get_2 (set `/Game/Blueprints/BP_SceneRotator.MotorSpeed` _output_get (`self.BP_SceneRotator`)))
  (`KismetSystemLibrary.PrintString` (`KismetStringLibrary.Concat_StrStr` "MotorSpeed :" (`KismetStringLibrary.Conv_DoubleToString` _output_get_2))))

(fn `UserConstructionScript`)