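; BP_SceneRotator continuously spins a set of scene components around their local roll axis.
; Each Tick loops over the SceneComponents array and adds a local rotation of MotorSpeed scaled by world delta seconds, keeping the spin frame-rate independent.
; The first component tag sets the direction: "Right" gives the positive product, and any other value negates it.
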(event `self.ReceiveTick`
  (params (DeltaSeconds :type "Float (single-precision)"))
  (for _array_element (`self.SceneComponents`)
    (if (== (`|GetArrayItem` (`ActorComponent.ComponentTags` _array_element)) "Right")
      (`SceneComponent.K2_AddLocalRotation` _array_element (`KismetMathLibrary.MakeRotator` (* (`GameplayStatics.GetWorldDeltaSeconds`) (`self.MotorSpeed`))) false false)
      (else
        (`SceneComponent.K2_AddLocalRotation` _array_element (`KismetMathLibrary.MakeRotator` (* (* (`GameplayStatics.GetWorldDeltaSeconds`) (`self.MotorSpeed`)) -1.0)) false false)))))